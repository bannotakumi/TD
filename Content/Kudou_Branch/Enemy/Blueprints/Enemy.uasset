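; Enemy spawner Blueprint that keeps spawning random AI enemies at its own location and rotation.
; From BeginPlay, a random delay of several seconds precedes spawning a pawn class picked at random from the Pawn array, running the BT_EnemyAI behavior tree.
; After each spawn, a short for loop wires back into that Delay, so the cycle repeats with no exit condition.
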(event EventBeginPlay
  (Utilities|FlowControl|Delay (Math|Random|RandomFloatinRange 5.0 1e+01) :!label _label)
  (AI|SpawnAIFromClass (Utilities|Array|Get(acopy) (Variables|Default|GetPawn) (Math|Random|RandomIntegerinRange 0 (stale _result))) "/Game/Kudou_Branch/Enemy/Blueprints/BT_Assets/BT_EnemyAI.BT_EnemyAI" (Transformation|GetActorLocation) (Transformation|GetActorRotation) false 0)
  (for _index (range 0 3)
    (goto _label)))

(fn ConstructionScript)