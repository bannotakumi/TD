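; AI_Enemy is an enemy pawn Blueprint that relays AI perception results to its AIC_Enemy controller.
; Sensing an actor cancels the lost-target timer and sets the target and line-of-sight keys through the controller.
; Losing it clears line of sight immediately but keeps the target until a five-second timer expires.
; A random-wander event using navigation points exists, but its timer setup is disconnected.
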(event OnTargetPerceptionUpdated(AIPerception)
  (params (Actor :type Actor%20Object%20Reference) (Stimulus :type AI%20Stimulus%20Structure))
  (Variables|Default|SetPerceivedActor Actor)
  (if (.bSuccessfullySensed (Utilities|Struct|BreakAIStimulus Stimulus))
    (Utilities|Time|ClearandInvalidateTimerbyHandle (Variables|Default|GetTargetLostTimer))
    (Default|UpdateTargetActorKey (.AsAIC%20Enemy (Utilities|Casting|CastToAIC_Enemy (Pawn|GetController))) (Variables|Default|GetPerceivedActor))
    (Default|UpdateHasLineOfSightKey (.AsAIC%20Enemy (Utilities|Casting|CastToAIC_Enemy (Pawn|GetController))) true)
    (else
      (bind _returnvalue (Utilities|Time|SetTimerbyEvent (delegate Custom|TargetLost) 5.0))
      (Variables|Default|SetTargetLostTimer _returnvalue)
      (Default|UpdateHasLineOfSightKey (.AsAIC%20Enemy (Utilities|Casting|CastToAIC_Enemy (Pawn|GetController))) false))))

(event Custom|RandomWander
  ;[1 1 1] ランダムに動くAI
  (AI|Navigation|SimpleMovetoLocation (Pawn|GetController) (.RandomLocation (AI|Navigation|GetRandomReachablePointinRadius (Transformation|GetActorLocation) 1e+03 0 0))))

(event Custom|TargetLost
  (Variables|Default|SetPerceivedActor 0)
  (Default|UpdateTargetActorKey (.AsAIC%20Enemy (Utilities|Casting|CastToAIC_Enemy (Pawn|GetController)))))

(event EventBeginPlay
  ;[1 1 1] ランダムに動くAI
)

(fn ConstructionScript)