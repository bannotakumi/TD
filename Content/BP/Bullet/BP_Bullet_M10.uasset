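; BP_Bullet_M10 is a bullet projectile actor that flies in a straight line and disappears on impact.
; A Rotation event sets its travel vector by rotating WorldVec with the supplied bullet rotation plus a 90-degree offset, then scaling by Speed.
; Tick moves it by that vector each frame with a sweep and no delta-time scaling.
; Hit spawns the P_ky_hit2 particle effect and destroys the bullet, applying no damage itself.
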(event EventBeginPlay)

(event Collision|EventActorBeginOverlap
  (params (OtherActor :type Actor%20Object%20Reference)))

(event EventTick
  (params (DeltaSeconds :type Float%20%28single-precision%29))
  (Transformation|SetActorLocationAndRotation (+ (Transformation|GetActorLocation) (Variables|Default|GetWorld_Vec)) "0, 0, 0" true))

(event Collision|EventHit
  (params (MyComp :type Primitive%20Component%20Object%20Reference) (Other :type Actor%20Object%20Reference) (OtherComp :type Primitive%20Component%20Object%20Reference) (bSelfMoved :type Boolean) (HitLocation :type Vector :default "0, 0, 0") (HitNormal :type Vector :default "0, 0, 0") (NormalImpulse :type Vector :default "0, 0, 0") (Hit :type Hit%20Result%20Structure%20%28by%20ref%29))
  (Effects|SpawnEmitteratLocation "/Game/Resources/GunEffects/P_ky_hit2.P_ky_hit2" HitLocation)
  (Actor|DestroyActor))

(event EventRotation
  (params (Bullet_Rot :type Rotator :default "0, 0, 0"))
  (Variables|Default|SetWorld_Vec (* (Math|Vector|RotateVector (Variables|Default|GetWorld_Vec) (Math|Rotator|CombineRotators "0.000000,90.000000, 0" Bullet_Rot)) (Variables|Default|GetSpeed))))

(fn ConstructionScript)