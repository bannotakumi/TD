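; VR AK-47 actor that attaches to left or right hand sockets on pickup and fires automatically while used.
; Tick runs a fire-rate timer, spawning bullets and muzzle flash at the muzzle socket until ammo runs out.
; Magazine events refill or empty the ammo, dropping a spawned empty magazine.
; Hitting "Ground" returns the gun to HiddenPlayerBody, and the capacitive trigger toggles the widget-interaction debug line as a laser pointer.
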(event OnComponentHit(SkeletalMeshComponent)
  (params (HitComponent :type Primitive%20Component%20Object%20Reference) (OtherActor :type Actor%20Object%20Reference) (OtherComp :type Primitive%20Component%20Object%20Reference) (NormalImpulse :type Vector :default "0, 0, 0") (Hit :type Hit%20Result%20Structure%20%28by%20ref%29))
  ;[1 1 1] 地面に落ちたら自分を所定の位置に戻す
  ;;[1 1 1] 地面(TagがGround)に当たったら
  ;;;[1 1 1] オブジェクトのnullチェック
  (if (Utilities|IsValid OtherActor)
    (if (Actor|ActorHasTag OtherActor "Ground")
      (Variables|Default|SetteleportCheck true))))

(event EventBeginPlay)

(event EventDetach
  ;[1 1 1] 手放す
  (Transformation|DetachFromActor "KeepWorld" "KeepWorld" "KeepWorld"))

(event EventAddMagazine
  ;[1 1 1] マガジンの追加
  (if (not (Variables|Default|GetmagazineChack))
    (Variables|Default|SetBullets (Variables|Default|GetmaxBullets))
    ;;[1 1 1] マガジン装着時のSE
    ;;;[1 1 1] リロード音指定
    (Audio|SpawnSoundatLocation "/Game/Weapons/Sounds/AssultRifle/wav/sw_Wep_Reload_AR.sw_Wep_Reload_AR" (Transformation|GetActorLocation) "0, 0, 0" 1.0 1.0 0.0 0 0 false)
    (Variables|Default|SetmagazineChack true)))

(event EventTick
  (params (DeltaSeconds :type Float%20%28single-precision%29))
  (bind _usesound (Variables|コンポーネント|GetUseSound))
  (bind _skeletalmeshcomponent (Variables|SkeletalMeshActor|GetSkeletalMeshComponent))
  (bind _returnvalue (Transformation|GetSocketTransform _skeletalmeshcomponent "b_gun_muzzleflash" "RTS_World"))
  ;[1 1 1] Update
  ;;[1 1 1] レーザーポインターの可視化
  (Variables|/Script/UMG.WidgetInteractionComponent|SetbShowDebug (Variables|Default|GetWidgetInteraction) (Variables|Default|GetlaserShowDebug))
  (if (Variables|Default|GetteleportCheck)
    ;;[1 1 1] 位置を常にHMDに合わせる
    ;;;[1 1 1] 銃の回転
    (Transformation|SetActorRotation (Variables|Default|GetaddGunSetRot))
    ;;;[1 1 1] 位置をワールドからローカルに変更
    (Transformation|SetActorLocation (Variables|Default|GetaddGunSetTrans) false false)
    ;;;[1 1 1] HiddenPlayerBodyへ親子付け
    (Transformation|AttachActorToActor self (Variables|Default|GetHiddenPlayerBody) "None" "KeepRelative" "KeepRelative" "KeepRelative" true)
    (Variables|Default|SetteleportCheck false)
    (Physics|SetSimulatePhysics (Variables|SkeletalMeshActor|GetSkeletalMeshComponent) false))
  (bind _output_get (Variables|Default|SetBulletTimer (- (Variables|Default|GetBulletTimer) DeltaSeconds)))
  ;;[1 1 1] マガジンの残弾チェック
  (bind _bulletchack (CallFunction|MagazineCheck))
  (if _bulletchack
    (Variables|Default|SetGun_Rotation (Transformation|GetActorRotation))
    ;;[1 1 1] 銃を連射中か否か
    (if (Variables|Default|GetBulletShotCheck)
      ;;[1 1 1] 銃の連射感覚タイマー
      (if (> 0.0 _output_get)
        ;;[1 1 1] タイマー初期化
        (Variables|Default|SetBulletTimer 0.05)
        ;;[1 1 1] 弾発射
        ;;;[1 1 1] 弾の指定
        (bind _returnvalue_2 (Game|SpawnActorfromClass "/Game/BP/Bullet/BP_Bullet_AK47.BP_Bullet_AK47_C" _returnvalue "Undefined" 0 0))
        (CallFunction|ShotBullet _returnvalue_2)
        (bind _output_get_2 (Variables|Default|SetSocketTransform _returnvalue))
        ;;;[1 1 1] 発射時のエフェクト指定
        (Effects|SpawnEmitteratLocation "/Game/Resources/GunEffects/P_Flash.P_Flash" (.location _output_get_2) (.rotation _output_get_2) "0.030000,0.030000,0.030000")
        ;;[1 1 1] 残弾を減らす
        (Variables|Default|SetBullets (- (Variables|Default|GetBullets) 1))))
    (else
      ;;[1 1 1] 残弾が切れたら音も消す
      (Utilities|IsValid _usesound
        (:Is%20Valid
          (Audio|Components|Audio|Stop _usesound))))))

(event EventPickup
  (params (AttachTo :type Scene%20Component%20Object%20Reference) (SocketName :type Name :default "None"))
  (bind _rootcomponent (Variables|Transformation|GetRootComponent))
  (bind _skeletalmeshcomponent (Variables|SkeletalMeshActor|GetSkeletalMeshComponent))
  ;[1 1 1] 持った時の音指定
  (Audio|SpawnSoundatLocation "/Game/Weapons/Sounds/AssultRifle/wav/sw_Wep_AR_Equip_02.sw_Wep_AR_Equip_02" (Transformation|GetActorLocation) "0, 0, 0" 1.0 1.0 0.0 0 0)
  (Physics|SetSimulatePhysics _skeletalmeshcomponent false)
  (if (Utilities|Name|Equal(Name) SocketName "Right")
    (Transformation|AttachComponentToComponent _rootcomponent AttachTo "Ak_Socket_Right" "KeepWorld" "KeepWorld" "KeepWorld" false)
    (else
      (Transformation|AttachComponentToComponent _rootcomponent AttachTo "Ak_Socket_Left" "KeepWorld" "KeepWorld" "KeepWorld" false)))
  (Transformation|SetRelativeLocationAndRotation _skeletalmeshcomponent "0.000000,-2.000000,-1.000000" "0, 0, 0" false false)
  (Variables|Default|SetteleportCheck false))

(event EventElectrostaticTrigger
  (params (triggerTouth :type Boolean))
  ;[1 1 1] 静電容量トリガーに触れたとき
  (Variables|Default|SetlaserShowDebug triggerTouth))

(event EventDrop
  (Physics|SetSimulatePhysics (Variables|SkeletalMeshActor|GetSkeletalMeshComponent) true)
  (Transformation|DetachFromActor "KeepWorld" "KeepWorld" "KeepWorld"))

(event Collision|EventActorBeginOverlap
  (params (OtherActor :type Actor%20Object%20Reference)))

(event EventDropMagazine
  ;[1 1 1] マガジンを落とす
  (if (Variables|Default|GetmagazineChack)
    (Variables|Default|SetBullets 0)
    ;;[1 1 1] マガジンドロップ時のSE
    ;;;[1 1 1] マガジンを落とした時の音指定
    (Audio|SpawnSoundatLocation "/Game/Weapons/Sounds/AssultRifle/wav/sw_Wep_AR_Equip_02.sw_Wep_AR_Equip_02" (Transformation|GetActorLocation) "0, 0, 0" 1.0 1.0 0.0 0 0 false)
    ;;[1 1 1] マガジンの生成
    ;;;[1 1 1] 生成するマガジンを指定
    (Game|SpawnActorfromClass "/Game/BP/Magazine/MagazineEmpty_AK47.MagazineEmpty_AK47_C" (Transformation|GetSocketTransform (Variables|SkeletalMeshActor|GetSkeletalMeshComponent) "b_rifleMag" "RTS_World") "Undefined" 0 0)
    (Variables|Default|SetmagazineChack false)))

(event EventUse
  ;[1 1 1] 銃声
  (bind _bulletchack (CallFunction|MagazineCheck))
  (if _bulletchack
    ;;[1 1 1] 撃った時の音
    (bind _returnvalue (Audio|SpawnSoundatLocation "/Game/Resources/GunSounds/AK47.AK47" (Transformation|GetActorLocation) "0, 0, 0" 1.0 1.0 0.0 0 0 false))
    (Variables|コンポーネント|SetUseSound _returnvalue)
    (Variables|Default|SetBulletShotCheck true)))

(event EventUnUse
  (bind _usesound (Variables|コンポーネント|GetUseSound))
  ;[1 1 1] 銃を撃っていない状態
  (Utilities|IsValid _usesound
    (:Is%20Valid
      (Audio|Components|Audio|Stop _usesound)
      (Variables|Default|SetBulletShotCheck false))))

(fn ConstructionScript)

(fn GetPickGunRotation
  (return (Variables|Default|GetGun_Rotation)))

(fn ShotBullet
  (params (Bullet :type I%20BP%20Bullet%20Interface))
  (Default|Rotation Bullet (Variables|Default|GetGun_Rotation)))

(fn MagazineCheck
  ;[1 1 1] 残弾があればtrue,なければfalse
  (return (> (Variables|Default|GetBullets) 0)))

(fn GetGunTag
  (return "AK47"))

(fn InMagCheck
  (return (Variables|Default|GetmagazineChack)))