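; Gate actor with hit points and an on-screen HP bar, apparently a target for enemies.
; BeginPlay creates the GateHPbar widget from GateHP, and Tick passes it the actor's location to update its position.
; AnyDamage sets GateHP to Damage minus GateHP (operands appear reversed) and notifies the bar.
; The Gate component's hit event checks for the Enemy tag but does nothing yet.
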(event OnComponentHit(Gate)
  (params (HitComponent :type Primitive%20Component%20Object%20Reference) (OtherActor :type Actor%20Object%20Reference) (OtherComp :type Primitive%20Component%20Object%20Reference) (NormalImpulse :type Vector :default "0, 0, 0") (Hit :type Hit%20Result%20Structure%20%28by%20ref%29))
  ;[1 1 1] 敵からのダメージ処理
  (if (Actor|ActorHasTag OtherActor "Enemy")
    _))

(event EventBeginPlay
  (bind _returnvalue (UserInterface|CreateWidget "/Game/Moritaki_Branch/GateHPbar.GateHPbar_C" 0 (Variables|Default|GetGateHP)))
  (bind _output_get (Variables|Default|SetHPbar _returnvalue))
  (UserInterface|Viewport|AddtoViewport _output_get 0))

(event Game|Damage|EventAnyDamage
  (params (Damage :type Float%20%28single-precision%29) (DamageType :type Damage%20Type%20Object%20Reference) (InstigatedBy :type Controller%20Object%20Reference) (DamageCauser :type Actor%20Object%20Reference))
  (Variables|Default|SetGateHP (- Damage (Variables|Default|GetGateHP)))
  (Default|OnTakeDamage (Variables|Default|GetHPbar) Damage))

(event EventTick
  (params (DeltaSeconds :type Float%20%28single-precision%29))
  (bind _hpbar (Variables|Default|GetHPbar)
    (:then
      (Default|UpdateUILocation _hpbar (Transformation|GetActorLocation)))
    (:else)))

(fn ConstructionScript)